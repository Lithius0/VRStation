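; BP_ShadowDisplay is a prop actor that builds a "shadow display" copy of another actor from its static meshes.
; CreateFromActor adds a StaticMeshComponent for each of the source's, copying mesh and relative transform and setting M_ShadowDisplay on the first material slot.
; The copies start hidden, and the actor disables collision and scales slightly larger than unit size.
; Nothing in this Blueprint calls the function or reveals the copies.
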(event EventBeginPlay)

(event Collision|EventActorBeginOverlap
  (params (OtherActor :type Actor%20Object%20Reference)))

(event EventTick
  (params (DeltaSeconds :type Float%20%28single-precision%29)))

(fn ConstructionScript)

(fn CreatefromActor
  (params (Actor :type Actor%20Object%20Reference))
  (for _array_element (Actor|GetComponentsByClass "/Script/Engine.StaticMeshComponent")
    (bind _asstatic_mesh_component (Utilities|Casting|CastToStaticMeshComponent _array_element))
    (bind _returnvalue (Game|AddComponentbyClass "/Script/Engine.StaticMeshComponent" false (Transformation|GetRelativeTransform _asstatic_mesh_component)))
    (Utilities|FlowControl|Sequence
      (:then_0
        (Components|StaticMesh|SetStaticMesh _returnvalue (Variables|/Script/Engine.StaticMeshComponent|GetStaticMesh _asstatic_mesh_component)))
      (:then_1
        (Rendering|Material|SetMaterial _returnvalue 0 "/Game/Props/M_ShadowDisplay.M_ShadowDisplay"))
      (:then_2
        (Rendering|SetVisibility _returnvalue false false))
      (:then_3
        (Collision|SetActorEnableCollision false))
      (:then_4
        (Transformation|SetActorScale3D "1.100000,1.100000,1.100000")))))