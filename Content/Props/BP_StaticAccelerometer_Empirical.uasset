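; BP_StaticAccelerometer_Empirical is a prop that measures its own acceleration in G and shows it on a text display.
; At BeginPlay it binds its root mesh to the main space station's torus through a physics constraint.
; Tick accumulates time and, each sampling interval, derives acceleration from the change in velocity rather than any analytic formula, smoothing it with a weighted moving average before display.
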(event EventBeginPlay
  ;[1 1 1] Binding the accelerometer to station
  (bind _outactors (Actor|GetAllActorsOfClass "/Game/Station/BP_SpaceStation.BP_SpaceStation_C"))
  (bind _array_element (Utilities|Array|ForEachLoopwithBreak _outactors)
    (:LoopBody
      (if (Variables|/Game/Station/BP_SpaceStation.BP_SpaceStation_C|GetIsMainStation _array_element)
        (Class|PhysicsConstraintComponent|SetConstrainedComponents (Variables|Default|GetPhysicsConstraint) (Variables|Default|GetRootMesh) "None" (Variables|/Game/Station/BP_SpaceStation.BP_SpaceStation_C|GetTorus _array_element) "None")))))

(event EventTick
  (params (DeltaSeconds :type Float%20%28single-precision%29))
  (bind _returnvalue (Transformation|GetVelocity))
  (bind _output_get (Variables|Default|SetdebounceTime (+ DeltaSeconds (Variables|Default|GetdebounceTime))))
  (if (> _output_get (Variables|Default|GetsamplingRate))
    (Variables|Default|SetdebounceTime 0.0)
    (bind _output_get_2 (Variables|Default|SetlastAcceleration (Class|KismetMathLibrary|WeightedMovingAverageFloat (/ (Math|Vector|VectorLength (/ (- (Variables|Default|GetlastVelocity) _returnvalue) (Variables|Default|GetsamplingRate))) 980.664978) (Variables|Default|GetlastAcceleration) 1e+01)))
    (Rendering|Components|TextRender|SetText (Variables|Default|GetAccelerationDisplay) (Utilities|Text|ToText(Float) _output_get_2 "HalfFromZero" false true 1 2 2 2)) ; Display
    (Variables|Default|SetlastVelocity _returnvalue)))

(fn ConstructionScript)

(fn NewFunction0)