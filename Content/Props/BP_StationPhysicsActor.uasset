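; Physics prop for a space station that drifts with the main station's motion and can be held in VR.
; Tick applies quadratic drag toward the station's point velocity at the prop, with an arrow visualizing the force.
; While held, it also applies a force toward the holding component, damped by station-relative velocity.
; Pickup and Drop toggle attachment and Pawn collision.
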(event EventTick
  (params (DeltaSeconds :type Float%20%28single-precision%29))
  (bind _arrow (Variables|Default|GetArrow))
  (bind _staticmesh (Variables|Default|GetStaticMesh))
  (Utilities|FlowControl|Sequence
    (:then_0
      ;[1 1 1] Moving relative to station
      (if (and (> (Variables|Default|GetDragCoefficient) 0.0) (Utilities|IsValid (Variables|Default|GetSpaceStation))) ; If we don't want velocity to match, don't bother doing the math
        (bind _returnvalue (Physics|GetPhysicsLinearVelocity _staticmesh "None"))
        (bind _returnvalue_2 (Class|PrimitiveComponent|GetPhysicsLinearVelocityatPoint (Variables|/Game/Station/BP_SpaceStation.BP_SpaceStation_C|GetRoot (Variables|Default|GetSpaceStation)) (Transformation|GetWorldLocation _staticmesh) "None"))
        (Physics|AddForce (Variables|Default|GetStaticMesh) (* (* (- _returnvalue_2 _returnvalue) (Math|Vector|VectorLength (- _returnvalue_2 _returnvalue))) (Variables|Default|GetDragCoefficient)) "None" false)
        ;[1 1 1] Draw the debug arrows
        (Transformation|SetWorldRotation _arrow (Math|Rotator|FindLookatRotation (Math|Vector|MakeVector 0.0 0.0 0.0) (* (* (- _returnvalue_2 _returnvalue) (Math|Vector|VectorLength (- _returnvalue_2 _returnvalue))) (Variables|Default|GetDragCoefficient))) false false)
        (Transformation|SetWorldScale3D _arrow (Math|Vector|MakeVector (/ (Math|Vector|VectorLength (* (* (- _returnvalue_2 _returnvalue) (Math|Vector|VectorLength (- _returnvalue_2 _returnvalue))) (Variables|Default|GetDragCoefficient))) 1e+03) 1.0 1.0))))
    (:then_1
      ;[1 1 1] VR Holding
      (if (Variables|Default|GetHeld)
        (bind _force (|GetDesiredForceVector (Transformation|GetWorldLocation (Variables|Default|GetHeldTo))))
        (Physics|AddForce (Variables|Default|GetStaticMesh) (|ScaleForce _force DeltaSeconds) "None" false)))))

(event EventBeginPlay
  ;[1 1 1] Binding to Station
  (bind _outactors (Actor|GetAllActorsOfClass "/Game/Station/BP_SpaceStation.BP_SpaceStation_C"))
  (for _array_element _outactors
    (bind _asbp_space_station (Utilities|Casting|CastToBP_SpaceStation _array_element))
    (if (Variables|/Game/Station/BP_SpaceStation.BP_SpaceStation_C|GetIsMainStation _asbp_space_station)
      (Variables|Default|SetSpaceStation _asbp_space_station))))

(event EventPickup
  (params (AttachTo :type Scene%20Component%20Object%20Reference))
  (Transformation|AttachComponentToComponent AttachTo "None" "KeepWorld" "KeepWorld" "KeepWorld" false)
  (bind _asbp_player_character (Utilities|Casting|CastToBP_PlayerCharacter (Game|GetPlayerCharacter 0)))
  (Variables|Default|SetHeld true)
  (Variables|Default|SetHeldTo AttachTo)
  (Variables|Default|SetCharacter _asbp_player_character)
  (Collision|SetCollisionResponsetoChannel (Variables|Default|GetStaticMesh) "ECC_Pawn" "ECR_Ignore"))

(event EventDrop
  (Variables|Default|SetHeld false)
  (Collision|SetCollisionResponsetoChannel (Variables|Default|GetStaticMesh) "ECC_Pawn" "ECR_Block")
  (Transformation|DetachFromActor "KeepWorld" "KeepWorld" "KeepWorld"))

(fn ConstructionScript)