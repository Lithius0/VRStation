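; BP_StationLight_SSA is a station light prop that can be switched on and off.
; The construction script applies the LightIntensity variable to the point light and sets its units to candelas.
; TurnOn and TurnOff toggle that intensity and swap the LightGlow material between lit and unlit versions.
; The event graph holds only disabled default events, so switching relies on calls to those functions.
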(event EventBeginPlay
  (|CallParentFunction) ; This node is disabled and will not be called.\nDrag off pins to build functionality.
)

(event Collision|EventActorBeginOverlap
  (params (OtherActor :type Actor%20Object%20Reference)))

(event EventTick
  (params (DeltaSeconds :type Float%20%28single-precision%29)))

(fn ConstructionScript
  (|CallParentFunction)
  (Rendering|Components|Light|SetIntensity (Variables|Default|GetPointLight) (Variables|Light|GetLightIntensity))
  (Class|LocalLightComponent|SetIntensityUnits (Variables|Default|GetPointLight) "Candelas"))

(fn Turnon
  (Rendering|Components|Light|SetIntensity (Variables|Default|GetPointLight) (Variables|Light|GetLightIntensity))
  (Rendering|Material|SetMaterial (Variables|Default|GetLightGlow) 0 "/Game/Props/Lights/M_LightOn.M_LightOn"))

(fn TurnOff
  (Rendering|Components|Light|SetIntensity (Variables|Default|GetPointLight) 0.0)
  (Rendering|Material|SetMaterial (Variables|Default|GetLightGlow) 0 "/Game/Props/Lights/M_LightOff.M_LightOff"))