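; BP_CurvedTable is a table prop that builds its own curved exterior collision from a series of box components.
; Its Construction Script adds blocking query-and-physics boxes along an arc in the YZ plane, centred on an angle offset and rolled around X to follow the curve.
; Placement combines collider radius with each box's bounds extent, and adds the actor location's XY length to the height.
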(fn ConstructionScript
  (bind _collisionboxquantity (Variables|Default|GetCollisionBoxQuantity))
  (if (> _collisionboxquantity 0)
    (for _index (range 0 _collisionboxquantity)
      ;[1 1 1] Exterior Collider Creation
      (bind _returnvalue (AddComponent|AddBoxComponent false (Math|Transform|MakeTransform (Math|Vector|MakeVector 0.0 0.0 0.0) "0, 0, 0" (Math|Vector|MakeVector (Variables|Default|GetColliderDepth) (Variables|Default|GetColliderWidth) (Variables|Default|GetColliderHeight)))))
      (Collision|SetCollisionResponsetoAllChannels _returnvalue "ECR_Block")
      (Collision|SetCollisionEnabled _returnvalue "QueryAndPhysics")
      (Transformation|SetRelativeLocationAndRotation _returnvalue (Math|Vector|MakeVector 0.0 (* (Math|Trig|Cos(Degrees) (+ (* (Math|Conversions|ToFloat(Integer) (+ _index (/ _collisionboxquantity -2))) (Variables|Default|GetColliderAngleDifference)) (Variables|Default|GetAngleOffset))) (+ (.Z (Math|Vector|BreakVector (.BoxExtent (Collision|GetComponentBounds _returnvalue)))) (Variables|Default|GetColliderRadius))) (+ (* (+ (.Z (Math|Vector|BreakVector (.BoxExtent (Collision|GetComponentBounds _returnvalue)))) (Variables|Default|GetColliderRadius)) (Math|Trig|Sin(Degrees) (+ (* (Math|Conversions|ToFloat(Integer) (+ _index (/ _collisionboxquantity -2))) (Variables|Default|GetColliderAngleDifference)) (Variables|Default|GetAngleOffset)))) (Math|Vector|VectorLengthXY (Transformation|GetActorLocation)))) (Math|Rotator|MakeRotator (* -1 (* (Math|Conversions|ToFloat(Integer) (+ _index (/ _collisionboxquantity -2))) (Variables|Default|GetColliderAngleDifference))) 0.0 0.0) false false))))