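; Space station actor whose physics-driven Torus spins toward a target speed around Z.
; Tick applies mass-independent torque scaled by the angular velocity error and records the current speed, while GetSpinSpeed returns the Z spin.
; The construction script places point lights in a ring attached to the Torus.
; It also builds a ring of blocking box colliders, rotated and pushed outward by their depth to approximate the exterior.
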(event EventTick
  (params (DeltaSeconds :type Float%20%28single-precision%29))
  ;[1 1 1] Rotation
  (Class|PrimitiveComponent|AddTorqueinRadians (Variables|Default|GetTorus) (* (* (- (Math|Vector|MakeVector 0.0 0.0 (Variables|SpinSpeed|GetTargetSpeed)) (Class|PrimitiveComponent|GetPhysicsAngularVelocityinRadians (Variables|Default|GetTorus) "None")) (Variables|SpinSpeed|GetAcceleration)) DeltaSeconds) "None" true)
  (Variables|SpinSpeed|SetCurrentSpeed (Math|Vector|VectorLength (Class|PrimitiveComponent|GetPhysicsAngularVelocityinRadians (Variables|Default|GetTorus) "None"))))

(fn ConstructionScript
  (bind _collisionboxquantity (Variables|OutsideCollision|GetCollisionBoxQuantity))
  (bind _number_of_lights (Variables|Lighting|GetNumber%20of%20Lights))
  (bind _top_light_radius (Variables|Lighting|GetTop%20Light%20Radius))
  (Utilities|FlowControl|Sequence
    (:then_0
      (if (> _number_of_lights 0)
        (for _index (range 0 _number_of_lights)
          ;[1 1 1] Light Creation
          (bind _returnvalue (AddComponent|AddPointLightComponent false (Math|Conversions|ToTransform(Vector) (Math|Vector|MakeVector (* (Math|Trig|Cos(Radians) (+ (/ (* (Math|Conversions|ToFloat(Integer) _index) (Class|KismetMathLibrary|GetTAU)) (Math|Conversions|ToFloat(Integer) (Variables|Lighting|GetNumber%20of%20Lights))) (Variables|Lighting|GetOffset))) _top_light_radius) (* (Math|Trig|Sin(Radians) (+ (/ (* (Math|Conversions|ToFloat(Integer) _index) (Class|KismetMathLibrary|GetTAU)) (Math|Conversions|ToFloat(Integer) (Variables|Lighting|GetNumber%20of%20Lights))) (Variables|Lighting|GetOffset))) _top_light_radius) 0.0))))
          (Transformation|AttachComponentToComponent _returnvalue (Variables|Default|GetTorus) "None" "KeepRelative" "KeepRelative" "KeepRelative" true)
          (Rendering|Components|Light|SetIntensity _returnvalue (Variables|Lighting|GetIntensity))
          (Class|LocalLightComponent|SetIntensityUnits _returnvalue "Candelas")
          (Rendering|Components|Light|SetLightColor _returnvalue (Variables|Lighting|GetColor) true)
          (Class|PointLightComponent|SetSourceRadius _returnvalue (Variables|Lighting|GetLight%20Source%20Radius)))
        (if (> _collisionboxquantity 0) :!label _label
          (for _index_2 (range 0 _collisionboxquantity)
            ;[1 1 1] Exterior Collider Creation
            (bind _returnvalue_2 (AddComponent|AddBoxComponent false (Math|Transform|MakeTransform "0, 0, 0" "0, 0, 0" (Math|Vector|MakeVector (Variables|OutsideCollision|GetColliderDepth) (Variables|OutsideCollision|GetColliderWidth) (Variables|OutsideCollision|GetColliderHeight)))))
            (Collision|SetCollisionResponsetoAllChannels _returnvalue_2 "ECR_Block")
            (Collision|SetCollisionEnabled _returnvalue_2 "QueryAndPhysics")
            (Transformation|SetRelativeLocationAndRotation _returnvalue_2 (Math|Vector|MakeVector (* (Math|Trig|Cos(Degrees) (* _index_2 (/ 3.6e+02 (Math|Conversions|ToFloat(Integer) _collisionboxquantity)))) (+ (.X (Math|Vector|BreakVector (.BoxExtent (Collision|GetComponentBounds _returnvalue_2)))) (Variables|OutsideCollision|GetColliderRadius))) (* (+ (.X (Math|Vector|BreakVector (.BoxExtent (Collision|GetComponentBounds _returnvalue_2)))) (Variables|OutsideCollision|GetColliderRadius)) (Math|Trig|Sin(Degrees) (* _index_2 (/ 3.6e+02 (Math|Conversions|ToFloat(Integer) _collisionboxquantity))))) 0.0) (Math|Rotator|MakeRotator 0.0 0.0 (* _index_2 (/ 3.6e+02 (Math|Conversions|ToFloat(Integer) _collisionboxquantity)))) false false)
            (Utilities|Array|Add (Variables|OutsideCollision|GetCollisionBoxes) _returnvalue_2)))))
    (:then_1
      (goto _label))))

(fn GetSpinSpeed
  (return (.Z (Math|Vector|BreakVector (Class|PrimitiveComponent|GetPhysicsAngularVelocityinRadians (Variables|Default|GetTorus) "None")))))