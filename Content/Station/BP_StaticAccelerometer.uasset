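; BP_StaticAccelerometer is a station accelerometer that shows its own acceleration in G on AccelerationDisplay.
; Each Tick it divides the change in actor velocity by delta time, converts cm/s² to G and stores the velocity for the next frame.
; The value goes through a weighted moving average, but its weight of 5 clamps to 1, so the readout is effectively unsmoothed.
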(event EventTick
  (params (DeltaSeconds :type Float%20%28single-precision%29))
  (bind _returnvalue (Transformation|GetVelocity))
  (Variables|Default|SetlastAcceleration (Class|KismetMathLibrary|WeightedMovingAverageFloat (/ (Math|Vector|VectorLength (/ (- (Variables|Default|GetlastVelocity) _returnvalue) DeltaSeconds)) 980.664978) (Variables|Default|GetlastAcceleration) 5.0))
  (Rendering|Components|TextRender|SetText (Variables|Default|GetAccelerationDisplay) (Utilities|Text|ToText(Float) (Class|KismetMathLibrary|WeightedMovingAverageFloat (/ (Math|Vector|VectorLength (/ (- (Variables|Default|GetlastVelocity) _returnvalue) DeltaSeconds)) 980.664978) (Variables|Default|GetlastAcceleration) 5.0) "HalfFromZero" false true 1 1 2 2))
  (Variables|Default|SetlastVelocity _returnvalue))

(fn ConstructionScript)

(fn NewFunction0)