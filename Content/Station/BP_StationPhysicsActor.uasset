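; Physics actor that gets dragged along with the motion of the main space station.
; On BeginPlay it finds the BP_SpaceStation flagged IsMainStation and stores a reference to it.
; Each tick it applies a force proportional to the gap between its velocity and the station Torus's velocity at its location, scaled by DragCoefficient.
; An Arrow component visualizes that force's direction and magnitude.
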(event EventTick
  (params (DeltaSeconds :type Float%20%28single-precision%29))
  (bind _arrow (Variables|Default|GetArrow))
  (bind _staticmesh (Variables|Default|GetStaticMesh))
  ;[1 1 1] Moving relative to station
  (if (and (> (Variables|Default|GetDragCoefficient) 0.0) (Utilities|IsValid (Variables|Default|GetSpaceStation))) ; If we don't want velocity to match, don't bother doing the math
    (bind _returnvalue (Physics|GetPhysicsLinearVelocity _staticmesh "None"))
    (bind _returnvalue_2 (Class|PrimitiveComponent|GetPhysicsLinearVelocityatPoint (Variables|/Game/Station/BP_SpaceStation.BP_SpaceStation_C|GetTorus (Variables|Default|GetSpaceStation)) (Transformation|GetWorldLocation _staticmesh) "None"))
    (Physics|AddForce (Variables|Default|GetStaticMesh) (* (- _returnvalue_2 _returnvalue) (Variables|Default|GetDragCoefficient)) "None" false)
    (Transformation|SetWorldRotation _arrow (Math|Rotator|FindLookatRotation (Math|Vector|MakeVector 0.0 0.0 0.0) (* (- _returnvalue_2 _returnvalue) (Variables|Default|GetDragCoefficient))) false false)
    (Transformation|SetWorldScale3D _arrow (Math|Vector|MakeVector (/ (Math|Vector|VectorLength (* (- _returnvalue_2 _returnvalue) (Variables|Default|GetDragCoefficient))) 1e+03) 1.0 1.0))))

(event EventBeginPlay
  ;[1 1 1] Binding to Station
  (bind _outactors (Actor|GetAllActorsOfClass "/Game/Station/BP_SpaceStation.BP_SpaceStation_C"))
  (for _array_element _outactors
    (bind _asbp_space_station (Utilities|Casting|CastToBP_SpaceStation _array_element))
    (if (Variables|/Game/Station/BP_SpaceStation.BP_SpaceStation_C|GetIsMainStation _asbp_space_station)
      (Variables|Default|SetSpaceStation _asbp_space_station)
      (Development|PrintString "Object bound to Station"))))

(fn ConstructionScript)